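; Base enemy Blueprint for a retro FPS, drawing enemies as eight-directional billboard flipbook sprites and running a behavior tree on BeginPlay.
; The Billboard event yaws the sprite toward the camera, then uses forward and right dot products against the player direction to pick idle or walking flipbooks.
; Damage briefly pauses facing updates for a hurt animation, while death stops AI, disables capsule collision and plays dying, then dead flipbooks.
; Melee and ranged attack events are empty.
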(event `self.ReceiveBeginPlay`
  (bind _asbp_osfpsenemy_ai (cast `/Game/OldSchoolFPS/Blueprints/Enemies/AI/BP_OSFPSEnemyAI` (`self.GetController`)))
  (`AIController.RunBehaviorTree` _asbp_osfpsenemy_ai (`self.BehaviourTree`)))

(event `Billboard`
  (`self.SpriteFacePlayer`
    (:`Out`
      (if (not (or (`self.IsDead`) (`self.PauseAngleCalc`)))
        (`self.GetEnemyAngle`
          (:`Out`
            (`self.CheckIfWalking`
              (:`Out`
                (`self.CalculateFlipbook`)))))))))

(event `self.KillCharacter`
  (params (NewParam :type "InterchangeVolumeTextureFactoryNode Object Reference"))
  (bind _enemy (`self.Enemy`))
  (`parent.KillCharacter` null)
  (bind _asbp_osfpsenemy_ai (cast `/Game/OldSchoolFPS/Blueprints/Enemies/AI/BP_OSFPSEnemyAI` (`self.GetController`)))
  (`BrainComponent.StopLogic` (`AIController.BrainComponent` _asbp_osfpsenemy_ai) "")
  (set `self.IsDead` true)
  (`PrimitiveComponent.SetCollisionEnabled` (`self.CapsuleComponent`) "NoCollision")
  (`PaperFlipbookComponent.SetFlipbook` _enemy (`self.Dying`))
  (`KismetSystemLibrary.Delay` (`PaperFlipbookComponent.GetFlipbookLength` _enemy))
  (`PaperFlipbookComponent.SetFlipbook` (`self.Enemy`) (`self.Dead`)))

(event `self.TakeDamage`
  (params (CueData :type "GameplayCueParameters Structure"))
  (bind _enemy (`self.Enemy`))
  (`parent.TakeDamage` CueData)
  (if (not (`self.IsDead`))
    (set `self.PauseAngleCalc` true)
    (`PaperFlipbookComponent.SetFlipbook` _enemy (`self.Damaged`))
    (`KismetSystemLibrary.Delay` (`PaperFlipbookComponent.GetFlipbookLength` _enemy))
    (set `self.PauseAngleCalc` false)))

(event `MeleeAttack`)

(event `RangedAttack`)

(fn `SetFlipbook`
  (params (Walking :type "PaperFlipbook Object Reference") (Idle :type "PaperFlipbook Object Reference"))
  (bind _enemy (`self.Enemy`))
  (if (`self.IsWalking`)
    (`PaperFlipbookComponent.SetFlipbook` _enemy Walking)
    (else
      (`PaperFlipbookComponent.SetFlipbook` _enemy Idle))))

(fn `UserConstructionScript`
  (`parent.UserConstructionScript`))