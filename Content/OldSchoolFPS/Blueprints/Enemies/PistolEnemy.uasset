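; PistolEnemy is a ranged enemy Blueprint for an old-school FPS, built on a parent class and the Gameplay Ability System.
; RangedAttack plays a sound, activates an ability by tag and briefly reveals a point light as a flash.
; Tick calls Billboard every frame and plays a death sound once, guarded by a flag, when a monitored ability-system attribute drops to zero or below.
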(event `self.RangedAttack`
  (`GameplayStatics.PlaySound2D` "/Game/OldSchoolFPS/Audio/Enemy/rangedAttack.rangedAttack" 1.0 1.0 0.0 null null)
  (`AbilitySystemComponent.TryActivateAbilitiesByTag` (`self.AbilitySystemComponent`) (`self.Gameplay Tag Container`) false)
  (`SceneComponent.SetHiddenInGame` (`self.PointLight`) false false)
  (`KismetSystemLibrary.Delay` 0.2)
  (`SceneComponent.SetHiddenInGame` (`self.PointLight`) true false))

(event `self.ReceiveTick`
  (params (DeltaSeconds :type "Float (single-precision)"))
  (`self.Billboard`)
  (if (<= (`.ReturnValue` (`AbilitySystemBlueprintLibrary.GetFloatAttributeFromAbilitySystemComponent` (`self.AbilitySystemComponent`) (struct :`AttributeName` "Health" :`Attribute` "/Script/OldSchoolFPS.OSFPSAttributeSet:Health" :`AttributeOwner` "/Script/CoreUObject.Class'\"/Script/OldSchoolFPS.OSFPSAttributeSet\"'"))) 0.0)
    (if (not (`self.playedSound`))
      (`GameplayStatics.PlaySound2D` "/Game/OldSchoolFPS/Audio/Enemy/rangeedDead.rangeedDead" 1.0 1.0 0.0 null null)
      (set `self.playedSound` true))))

(fn `UserConstructionScript`
  (`parent.UserConstructionScript`))