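; BP_DoorRed is a sliding door that opens for the FPS player character, optionally gated by a keycard.
; Entering BoxColl opens it if it is unlocked or the character's KeyCards contain KeyNeeded, and leaving closes it again.
; The Position timeline lerps the door upward from the location cached at BeginPlay, and closing plays the same timeline in reverse.
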(event `self.ReceiveBeginPlay`
  (set `self.StartPos` (`SceneComponent.RelativeLocation` (`self.Door`))))

(event `self.ReceiveTick`
  (params (DeltaSeconds :type "Float (single-precision)")))

(event `self.BoxColl.OnComponentBeginOverlap`
  (params (OverlappedComponent :type "PrimitiveComponent Object Reference") (OtherActor :type "Actor Object Reference") (OtherComp :type "PrimitiveComponent Object Reference") (OtherBodyIndex :type Integer) (bFromSweep :type Boolean) (SweepResult :type "HitResult Structure (by ref)"))
  (bind _asbp_fpcc (cast `/Game/OldSchoolFPS/Blueprints/Player/BP_FPCC` OtherActor))
  (if (`self.Locked?`)
    (if (`KismetArrayLibrary.Array_Contains` (`/Game/OldSchoolFPS/Blueprints/Player/BP_FPCC.KeyCards` _asbp_fpcc) (`self.KeyNeeded`))
      (`self.OpenDoor`)
      (set `self.DoorOpened?` true))
    (else
      (`self.OpenDoor`)
      (set `self.DoorOpened?` true))))

(event `self.BoxColl.OnComponentEndOverlap`
  (params (OverlappedComponent :type "PrimitiveComponent Object Reference") (OtherActor :type "Actor Object Reference") (OtherComp :type "PrimitiveComponent Object Reference") (OtherBodyIndex :type Integer))
  (cast `/Game/OldSchoolFPS/Blueprints/Player/BP_FPCC` OtherActor)
  (if (`self.DoorOpened?`)
    (`self.CloseDoor`)
    (set `self.DoorOpened?` false)))

(event `OpenDoor`
  (bind _startpos (`self.StartPos`))
  (bind (_direction _speed) (`Timeline|Position` :!label _label)
    (:`Update`
      (`SceneComponent.K2_SetRelativeLocation` (`self.Door`) (`KismetMathLibrary.VLerp` _startpos (- _startpos (0.0 0.0 -450.0)) _speed) false false))))

(event `CloseDoor`
  (goto _label :!via `Reverse`))

(fn `UserConstructionScript`)