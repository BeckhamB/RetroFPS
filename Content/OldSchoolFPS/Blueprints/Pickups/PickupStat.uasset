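; Health or armour stat pickup for the old-school FPS, drawn as a Paper2D flipbook.
; The construction script uses pickup type and size to set the sprite, scale and matching gameplay tag.
; Two helper functions read an Ability System attribute and add or remove a player Full tag at 100, though nothing here calls them.
; Tick only defers to the parent, so any pickup handling lies outside this Blueprint.
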(event `self.ReceiveTick`
  (params (DeltaSeconds :type "Float (single-precision)"))
  (`parent.ReceiveTick` DeltaSeconds))

(fn `FullArmourCheck`
  (params (AbilitySystem :type "AbilitySystemComponent Object Reference"))
  (bind _pickuptag (`self.PickupTag`))
  (if (== (`.ReturnValue` (`AbilitySystemBlueprintLibrary.GetFloatAttributeFromAbilitySystemComponent` AbilitySystem (struct :`AttributeName` "Armour" :`Attribute` "/Script/OldSchoolFPS.OSFPSAttributeSet:Armour" :`AttributeOwner` "/Script/CoreUObject.Class'\"/Script/OldSchoolFPS.OSFPSAttributeSet\"'"))) 100.0)
    (`BlueprintGameplayTagLibrary.AddGameplayTag` _pickuptag (struct :`TagName` "Player.Armour.Full"))
    (else
      (`BlueprintGameplayTagLibrary.RemoveGameplayTag` _pickuptag (struct :`TagName` "Player.Armour.Full")))))

(fn `FullHealthCheck`
  (params (AbilitySystem :type "AbilitySystemComponent Object Reference"))
  (bind _pickuptag (`self.PickupTag`))
  (if (== (`.ReturnValue` (`AbilitySystemBlueprintLibrary.GetFloatAttributeFromAbilitySystemComponent` AbilitySystem (struct :`AttributeName` "Health" :`Attribute` "/Script/OldSchoolFPS.OSFPSAttributeSet:Health" :`AttributeOwner` "/Script/CoreUObject.Class'\"/Script/OldSchoolFPS.OSFPSAttributeSet\"'"))) 100.0)
    (`BlueprintGameplayTagLibrary.AddGameplayTag` _pickuptag (struct :`TagName` "Player.Health.Full"))
    (else
      (`BlueprintGameplayTagLibrary.RemoveGameplayTag` _pickuptag (struct :`TagName` "Player.Health.Full")))))

(fn `SetStatPickupFB`
  (bind _pickup (`self.Pickup`))
  (bind _pickup_2 (`self.Pickup`))
  (switch `/Game/OldSchoolFPS/Blueprints/Enums/ENUM_PickupType` (`self.PickupType`)
    (:`NewEnumerator0`
      (`PaperFlipbookComponent.SetFlipbook` _pickup "/Game/OldSchoolFPS/Flipbooks/Pickups/FB_ArmorPickup.FB_ArmorPickup")
      (switch `/Game/OldSchoolFPS/Blueprints/Enums/ENUM_PickupSize` (`self.PickupSize`)
        (:`NewEnumerator0`
          (`SceneComponent.SetRelativeScale3D` _pickup_2 (2.0 2.0 2.0))
          (set `self.PickupTag` (struct :`GameplayTags` (struct :`(TagName` "Pickup.Armour.Small")))))
        (:`NewEnumerator1`
          (`SceneComponent.SetRelativeScale3D` _pickup_2 (3.0 3.0 3.0))
          (set `self.PickupTag` (struct :`GameplayTags` (struct :`(TagName` "Pickup.Armour.Large")))))))
    (:`NewEnumerator1`
      (`PaperFlipbookComponent.SetFlipbook` _pickup "/Game/OldSchoolFPS/Flipbooks/Pickups/FB_HealthPickup.FB_HealthPickup")
      (switch `/Game/OldSchoolFPS/Blueprints/Enums/ENUM_PickupSize` (`self.PickupSize`)
        (:`NewEnumerator0`
          (`SceneComponent.SetRelativeScale3D` _pickup_2 (2.0 2.0 2.0))
          (set `self.PickupTag` (struct :`GameplayTags` (struct :`(TagName` "Pickup.Health.Small")))))
        (:`NewEnumerator1`
          (`SceneComponent.SetRelativeScale3D` _pickup_2 (3.0 3.0 3.0))
          (set `self.PickupTag` (struct :`GameplayTags` (struct :`(TagName` "Pickup.Health.Large")))))))))

(fn `UserConstructionScript`
  (`parent.UserConstructionScript`)
  (`self.SetStatPickupFB`))