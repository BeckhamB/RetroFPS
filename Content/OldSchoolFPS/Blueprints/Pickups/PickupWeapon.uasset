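; Weapon pickup actor for an old-school FPS that grants a weapon to the player on touch.
; The construction script sets the Pickup flipbook sprite from the WeaponToAcquire enum, covering pistol, launcher and shotgun, with an empty sprite for None.
; On overlap with a BP_FPCC character, it passes that weapon to the character's PickupWeapon and destroys itself.
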(event `self.ReceiveActorBeginOverlap`
  (params (OtherActor :type "Actor Object Reference"))
  (bind _asbp_fpcc (cast `/Game/OldSchoolFPS/Blueprints/Player/BP_FPCC` OtherActor))
  (`/Game/OldSchoolFPS/Blueprints/Player/BP_FPCC.PickupWeapon` _asbp_fpcc (`self.Weapon to Acquire`))
  (`self.K2_DestroyActor`))

(fn `UserConstructionScript`
  (bind _pickup (`self.Pickup`))
  (switch `/Game/OldSchoolFPS/Blueprints/Enums/ENUM_WeaponList` (`self.Weapon to Acquire`)
    (:`NewEnumerator0`
      (`PaperFlipbookComponent.SetFlipbook` _pickup null))
    (:`NewEnumerator1`
      (`PaperFlipbookComponent.SetFlipbook` _pickup "/Game/OldSchoolFPS/Flipbooks/Pickups/FB_pistol_pickup.FB_pistol_pickup"))
    (:`NewEnumerator2`
      (`PaperFlipbookComponent.SetFlipbook` _pickup "/Game/OldSchoolFPS/Flipbooks/Pickups/FB_LauncherPickups.FB_LauncherPickups"))
    (:`NewEnumerator3`
      (`PaperFlipbookComponent.SetFlipbook` _pickup "/Game/OldSchoolFPS/Flipbooks/Pickups/newShotgunPickup.newShotgunPickup"))))