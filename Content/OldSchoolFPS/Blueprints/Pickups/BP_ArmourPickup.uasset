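; Armour pickup Blueprint that grants its effect through the Gameplay Ability System when the player character overlaps it.
; On overlap with a BP_FPCC, it runs FullArmourCheck on that character's ability system component, then tries to activate abilities matching PickupTag.
; Only a successful activation calls ItemPickup on the character and destroys the actor, so a failed attempt leaves the pickup in place.
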(event `self.ReceiveActorBeginOverlap`
  (params (OtherActor :type "Actor Object Reference"))
  (`parent.ReceiveActorBeginOverlap` OtherActor)
  (bind _asbp_fpcc (cast `/Game/OldSchoolFPS/Blueprints/Player/BP_FPCC` OtherActor))
  (bind _returnvalue (`AbilitySystemBlueprintLibrary.GetAbilitySystemComponent` _asbp_fpcc))
  (`self.FullArmourCheck` _returnvalue)
  (bind _returnvalue_2 (`AbilitySystemComponent.TryActivateAbilitiesByTag` _returnvalue (`self.PickupTag`) false))
  (if _returnvalue_2
    (`/Game/OldSchoolFPS/Blueprints/Player/BP_FPCC.ItemPickup` _asbp_fpcc)
    (`self.K2_DestroyActor`)))

(fn `UserConstructionScript`
  (`parent.UserConstructionScript`))