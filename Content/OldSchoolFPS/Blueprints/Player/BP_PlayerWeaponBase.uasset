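; Base Blueprint for the player's weapon in an old-school FPS, drawn as a Paper2D flipbook.
; A scene capture renders only the flipbook, and BeginPlay stores its resting relative location.
; InitWeapon clears, hides and rescales the flipbook.
; WeaponBobbing plays the WeaponSway sequence while moving, otherwise stops it and interpolates the flipbook toward its resting location.
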(event `self.ReceiveBeginPlay`
  (`SceneCaptureComponent.ShowOnlyComponent` (`self.SceneCaptureComponent2D`) (`self.WeaponFlipbook`))
  (set `self.WeaponPosition` (`SceneComponent.RelativeLocation` (`self.WeaponFlipbook`))))

(event `/Game/OldSchoolFPS/Blueprints/Interfaces/I_PlayerWeapon.InitWeapon`
  (bind _weaponflipbook (`self.WeaponFlipbook`))
  (bind _weaponflipbook_2 (`self.WeaponFlipbook`))
  (`PaperFlipbookComponent.SetFlipbook` _weaponflipbook_2 null)
  (`SceneComponent.SetHiddenInGame` _weaponflipbook_2 true false)
  (`SceneComponent.K2_SetWorldTransform` _weaponflipbook (`KismetMathLibrary.MakeTransform` (`SceneComponent.K2_GetComponentLocation` _weaponflipbook) (`SceneComponent.K2_GetComponentRotation` _weaponflipbook) (0.1 0.1 0.1)) false false))

(event `WeaponBobbing`
  (params (IsMoving :type Boolean) (DeltaTime :type "Float (double-precision)"))
  (bind _weaponflipbook (`self.WeaponFlipbook`))
  (bind _sequenceplayer (`ActorSequenceComponent.SequencePlayer` (`self.WeaponSway`)))
  (if IsMoving
    (`MovieSceneSequencePlayer.Play` _sequenceplayer)
    (else
      (`MovieSceneSequencePlayer.Stop` _sequenceplayer)
      (`SceneComponent.K2_SetRelativeLocation` _weaponflipbook (`KismetMathLibrary.VInterpTo` (`SceneComponent.RelativeLocation` _weaponflipbook) (`self.WeaponPosition`) DeltaTime 10.0) false false))))

(fn `UserConstructionScript`)