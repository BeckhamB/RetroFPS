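; First-person player character for an old-school FPS, handling movement, look, weapons, pickups, damage, pause and game over on death.
; Weapons come from a data table, are stored in an inventory and spawn through a child actor component.
; Gameplay Ability System drives firing and ammo gain via tags chosen by weapon or pickup, and supplies attributes for health, armor and ammo.
; A HUD widget shows stats, keycards and timeline-driven screen flashes.
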(event `InputAction|FireWeapon`
  (params (Key :type "Key Structure"))
  ;[1 1 1] FireWeapon
  (:`Pressed`
    (`AbilitySystemComponent.TryActivateAbilitiesByTag` (`self.AbilitySystemComponent`) (`self.WeaponFireTagContainer`) false)))

(event `self.ReceiveBeginPlay`
  ;[1 1 1] Init
  (`parent.ReceiveBeginPlay`)
  (bind _returnvalue (`|CreateWidget` "/Game/OldSchoolFPS/Blueprints/Widgets/HUD.HUD_C"))
  (set `self.HUD` _returnvalue)
  (`UserWidget.AddToViewport` _returnvalue 0)
  (`KismetSystemLibrary.Delay` 0.0)
  (`self.UpdateUI`)
  (`self.InitWeapon` "/Game/OldSchoolFPS/Blueprints/Player/BP_PlayerWeaponBase.BP_PlayerWeaponBase_C")
  (`/Game/OldSchoolFPS/Blueprints/Widgets/HUD.SwitchWeapon` (`self.HUD`) "NewEnumerator0"))

(event `InputAction|SwitchPistol`
  (params (Key :type "Key Structure"))
  (:`Pressed`
    (if (`self.HasWeapon` "NewEnumerator1")
      (bind _weapondata (`self.GetWeaponFromDT` "NewEnumerator1"))
      (`self.Equip Weapon` _weapondata))))

(event `InputAxis|HorizontalMovement`
  (params (AxisValue :type "Float (single-precision)"))
  (bind (_returnvalue_roll _returnvalue_pitch _returnvalue_yaw) (`KismetMathLibrary.BreakRotator` (`self.GetControlRotation`)))
  ;[1 1 1] Inputs
  (`self.AddMovementInput` (`KismetMathLibrary.GetRightVector` (`KismetMathLibrary.MakeRotator` 0.0 0.0 _returnvalue_yaw)) AxisValue))

(event `InputAction|SwitchLauncher`
  (params (Key :type "Key Structure"))
  (:`Pressed`
    (if (`self.HasWeapon` "NewEnumerator2")
      (bind _weapondata (`self.GetWeaponFromDT` "NewEnumerator2"))
      (`self.Equip Weapon` _weapondata))))

(event `self.ReceiveTick`
  (params (DeltaSeconds :type "Float (single-precision)"))
  ;[1 1 1] Event Tick
  (bind _asbp_player_weapon_base (cast `/Game/OldSchoolFPS/Blueprints/Player/BP_PlayerWeaponBase` (`ChildActorComponent.ChildActor` (`self.Weapon`))))
  (`/Game/OldSchoolFPS/Blueprints/Player/BP_PlayerWeaponBase.WeaponBobbing` _asbp_player_weapon_base (> (`KismetMathLibrary.VSize` (`MovementComponent.Velocity` (`self.CharacterMovement`))) 0.0) DeltaSeconds)
  (if (<= (`.ReturnValue` (`AbilitySystemBlueprintLibrary.GetFloatAttributeFromAbilitySystemComponent` (`self.AbilitySystemComponent`) (struct :`AttributeName` "Health" :`Attribute` "/Script/OldSchoolFPS.OSFPSAttributeSet:Health" :`AttributeOwner` "/Script/CoreUObject.Class'\"/Script/OldSchoolFPS.OSFPSAttributeSet\"'"))) 0.0)
    (if (not (`self.playedDeathSound`))
      (`GameplayStatics.PlaySound2D` "/Game/OldSchoolFPS/Audio/Player/death.death" 1.0 1.0 0.0 null null)
      (set `self.playedDeathSound` true)
      (`GameplayStatics.OpenLevel` "GameOverMap"))))

(event `InputAxis|VerticalMovement`
  (params (AxisValue :type "Float (single-precision)"))
  (bind (_returnvalue_roll _returnvalue_pitch _returnvalue_yaw) (`KismetMathLibrary.BreakRotator` (`self.GetControlRotation`)))
  ;[1 1 1] Inputs
  (`self.AddMovementInput` (`KismetMathLibrary.GetForwardVector` (`KismetMathLibrary.MakeRotator` 0.0 0.0 _returnvalue_yaw)) AxisValue))

(event `InputAction|SwitchShotgun`
  (params (Key :type "Key Structure"))
  (:`Pressed`
    (if (`self.HasWeapon` "NewEnumerator3")
      (bind _weapondata (`self.GetWeaponFromDT` "NewEnumerator3"))
      (`self.Equip Weapon` _weapondata))))

(event `InputAxis|MouseLookHorizontal`
  (params (AxisValue :type "Float (single-precision)"))
  ;[1 1 1] Inputs
  (`self.AddControllerYawInput` AxisValue))

(event `Equip Weapon`
  (params (Weapon :type "/Game/OldSchoolFPS/Blueprints/Structs/ST_WeaponData Structure"))
  (bind _currentweapon_weaponname (break `/Game/OldSchoolFPS/Blueprints/Structs/ST_WeaponData` (`self.CurrentWeapon`)))
  (bind _currentweapon_weaponname_2 (break `/Game/OldSchoolFPS/Blueprints/Structs/ST_WeaponData` (`self.CurrentWeapon`)))
  ;[1 1 1] Equip Weapon
  (bind _output_get (set `self.CurrentWeapon` Weapon))
  (bind _weaponactor (`self.InitWeapon` (`.Weapon_5_5F37CFEE40413366AD89D4AB4AA70417` (break `/Game/OldSchoolFPS/Blueprints/Structs/ST_WeaponData` _output_get))))
  (bind _asbp_player_weapon_base (cast `/Game/OldSchoolFPS/Blueprints/Player/BP_PlayerWeaponBase` _weaponactor))
  (`MovieSceneSequencePlayer.Play` (`ActorSequenceComponent.SequencePlayer` (`/Game/OldSchoolFPS/Blueprints/Player/BP_PlayerWeaponBase.WeaponReady` _asbp_player_weapon_base)))
  (`/Game/OldSchoolFPS/Blueprints/Widgets/HUD.SwitchWeapon` (`self.HUD`) _currentweapon_weaponname)
  (`self.UpdateUI`)
  (switch `/Game/OldSchoolFPS/Blueprints/Enums/ENUM_WeaponList` _currentweapon_weaponname_2
    (:`NewEnumerator0`
      (set `self.WeaponFireTagContainer` (struct)))
    (:`NewEnumerator1`
      (set `self.WeaponFireTagContainer` (struct :`GameplayTags` (struct :`(TagName` "Player.Weapon.Pistol.Fire")))))
    (:`NewEnumerator2`
      (set `self.WeaponFireTagContainer` (struct :`GameplayTags` (struct :`(TagName` "Player.Weapon.Launcher.Fire")))))
    (:`NewEnumerator3`
      (set `self.WeaponFireTagContainer` (struct :`GameplayTags` (struct :`(TagName` "Player.Weapon.Shotgun.Fire")))))))

(event `InputAxis|MouseLookVertical`
  (params (AxisValue :type "Float (single-precision)"))
  ;[1 1 1] Inputs
  (`self.AddControllerPitchInput` AxisValue))

(event `SetVisiblityBlue`
  (`/Game/OldSchoolFPS/Blueprints/Widgets/HUD.SetBlueKeycardVisible` (`self.HUD`)))

(event `SetVisibiltyOrange`
  (`/Game/OldSchoolFPS/Blueprints/Widgets/HUD.SetOrangeKeycardVisible` (`self.HUD`)))

(event `SetVisibiltyRed`
  (`/Game/OldSchoolFPS/Blueprints/Widgets/HUD.SetRedKeycardVisible` (`self.HUD`)))

(event `PickupWeapon`
  (params (Weapon :type "/Game/OldSchoolFPS/Blueprints/Enums/ENUM_WeaponList Enum" :default "NewEnumerator0"))
  (bind (_weapondata _weaponfound) (`self.GetWeaponFromDT` Weapon))
  (if _weaponfound
    (bind _output_get (set `self.WeaponToPickup` _weapondata))
    (if (`self.HasWeapon` (`.WeaponName_3_853D30BD40417274EB9F7F9266644A8D` (break `/Game/OldSchoolFPS/Blueprints/Structs/ST_WeaponData` _output_get)))
      (bind (_weaponname _weapon _ammotype _ammosize) (break `/Game/OldSchoolFPS/Blueprints/Structs/ST_WeaponData` _output_get))
      (`self.AddAmmo` _ammotype _ammosize)
      (else
        (`self.AddWeapon`)))))

(event `self.TakeDamage`
  (params (CueData :type "GameplayCueParameters Structure"))
  ;[1 1 1] Take Damage
  (`parent.TakeDamage` CueData)
  (`self.UpdateUI`)
  (bind (_direction _alpha) (`Timeline|ScreenFlash` :!via `PlayFromStart`)
    (:`Update`
      (`/Game/OldSchoolFPS/Blueprints/Widgets/HUD.SetFlashColour` (`self.HUD`) (struct :`R` 1.0 :`B` 0.007763 :`A` 1.0) _alpha))
    (:`Finished`
      (`GameplayStatics.PlaySound2D` "/Game/OldSchoolFPS/Audio/Player/injured.injured" 1.0 1.0 0.0 null null))))

(event `AddAmmo`
  (params (AmmoType :type "/Game/OldSchoolFPS/Blueprints/Enums/ENUM_AmmoList Enum" :default "NewEnumerator0") (AmmoSize :type "/Game/OldSchoolFPS/Blueprints/Enums/ENUM_PickupSize Enum" :default "NewEnumerator0"))
  (switch `/Game/OldSchoolFPS/Blueprints/Enums/ENUM_AmmoList` AmmoType
    (:`NewEnumerator1`
      (`self.AddPistolBullets` AmmoSize))
    (:`NewEnumerator2`
      (`self.AddLauncherRockets` AmmoSize))
    (:`NewEnumerator3`
      (`self.AddShotgunShells` AmmoSize))))

(event `ItemPickup`
  ;[1 1 1] Pickups
  (`self.UpdateUI`)
  (bind (_direction _alpha) (`Timeline|Timeline` :!via `PlayFromStart`)
    (:`Update`
      (`/Game/OldSchoolFPS/Blueprints/Widgets/HUD.SetFlashColour` (`self.HUD`) (struct :`G` 0.378268 :`B` 1.0 :`A` 1.0) _alpha))))

(event `AddWeapon`
  (bind _weapontopickup (`self.WeaponToPickup`))
  (bind (_weaponname _weapon _ammotype _ammosize) (break `/Game/OldSchoolFPS/Blueprints/Structs/ST_WeaponData` _weapontopickup))
  (`KismetArrayLibrary.Array_Add` (`self.PlayerWeapons`) _weapontopickup)
  (`self.Equip Weapon` _weapontopickup)
  (`self.AddAmmo` _ammotype _ammosize))

(event `HealthPickup`
  ;[1 1 1] Pickups
  (`self.UpdateUI`)
  (bind (_direction _alpha) (`Timeline|Timeline_0` :!via `PlayFromStart`)
    (:`Update`
      (`/Game/OldSchoolFPS/Blueprints/Widgets/HUD.SetFlashColour` (`self.HUD`) (struct :`R` 0.010704 :`G` 1.0 :`A` 1.0) _alpha))))

(event `Key|P` :paused true
  (params (Key :type "Key Structure"))
  (bind _returnvalue (`GameplayStatics.GetPlayerController` 0))
  (:`Pressed`
    (if (`GameplayStatics.IsGamePaused`)
      (`/Engine/EditorBlueprintResources/StandardMacros.IsValid` (stale _returnvalue_2)
        (:`Is Valid`
          (`Widget.RemoveFromParent` (stale _returnvalue_2))
          (`GameplayStatics.SetGamePaused` false)
          (`WidgetBlueprintLibrary.SetInputMode_GameOnly` _returnvalue)
          (set `PlayerController.bShowMouseCursor` false _returnvalue)))
      (else
        (bind _returnvalue_2 (`|CreateWidget` "/Game/OldSchoolFPS/Blueprints/Widgets/PauseMenu.PauseMenu_C"))
        (`UserWidget.AddToViewport` _returnvalue_2 0)
        (`GameplayStatics.SetGamePaused` true)))))

(fn `AddLauncherRockets`
  (params (AmmoSize :type "/Game/OldSchoolFPS/Blueprints/Enums/ENUM_PickupSize Enum" :default "NewEnumerator0"))
  (if (not (>= (`.ReturnValue` (`AbilitySystemBlueprintLibrary.GetFloatAttributeFromAbilitySystemComponent` (`self.AbilitySystemComponent`) (struct :`AttributeName` "Rockets" :`Attribute` "/Script/OldSchoolFPS.OSFPSAttributeSet:Rockets" :`AttributeOwner` "/Script/CoreUObject.Class'\"/Script/OldSchoolFPS.OSFPSAttributeSet\"'"))) (`self.MaxRockets`)))
    (switch `/Game/OldSchoolFPS/Blueprints/Enums/ENUM_PickupSize` AmmoSize
      (:`NewEnumerator0`
        (set `self.AmmoGainTagCont` (struct :`GameplayTags` (struct :`(TagName` "Pickup.Ammo.Rockets.Small")))))
      (:`NewEnumerator1`
        (set `self.AmmoGainTagCont` (struct :`GameplayTags` (struct :`(TagName` "Pickup.Ammo.Rockets.Large"))))))
    (`AbilitySystemComponent.TryActivateAbilitiesByTag` (`self.AbilitySystemComponent`) (`self.AmmoGainTagCont`) true)
    (`self.ItemPickup`)))

(fn `AddPistolBullets`
  (params (AmmoSize :type "/Game/OldSchoolFPS/Blueprints/Enums/ENUM_PickupSize Enum" :default "NewEnumerator0"))
  (if (not (>= (`.ReturnValue` (`AbilitySystemBlueprintLibrary.GetFloatAttributeFromAbilitySystemComponent` (`self.AbilitySystemComponent`) (struct :`AttributeName` "Bullets" :`Attribute` "/Script/OldSchoolFPS.OSFPSAttributeSet:Bullets" :`AttributeOwner` "/Script/CoreUObject.Class'\"/Script/OldSchoolFPS.OSFPSAttributeSet\"'"))) (`self.MaxBullets`)))
    (switch `/Game/OldSchoolFPS/Blueprints/Enums/ENUM_PickupSize` AmmoSize
      (:`NewEnumerator0`
        (set `self.AmmoGainTagCont` (struct :`GameplayTags` (struct :`(TagName` "Pickup.Ammo.Pistol.Bullets.Small")))))
      (:`NewEnumerator1`
        (set `self.AmmoGainTagCont` (struct :`GameplayTags` (struct :`(TagName` "Pickup.Ammo.Pistol.Bullets.Large"))))))
    (`AbilitySystemComponent.TryActivateAbilitiesByTag` (`self.AbilitySystemComponent`) (`self.AmmoGainTagCont`) true)
    (`self.ItemPickup`)))

(fn `AddShotgunShells`
  (params (AmmoSize :type "/Game/OldSchoolFPS/Blueprints/Enums/ENUM_PickupSize Enum" :default "NewEnumerator0"))
  (if (not (>= (`.ReturnValue` (`AbilitySystemBlueprintLibrary.GetFloatAttributeFromAbilitySystemComponent` (`self.AbilitySystemComponent`) (struct :`AttributeName` "Shells" :`Attribute` "/Script/OldSchoolFPS.OSFPSAttributeSet:Shells" :`AttributeOwner` "/Script/CoreUObject.Class'\"/Script/OldSchoolFPS.OSFPSAttributeSet\"'"))) (`self.MaxShells`)))
    (switch `/Game/OldSchoolFPS/Blueprints/Enums/ENUM_PickupSize` AmmoSize
      (:`NewEnumerator0`
        (set `self.AmmoGainTagCont` (struct :`GameplayTags` (struct :`(TagName` "Pickup.Ammo.Shotgun.Shells.Small")))))
      (:`NewEnumerator1`
        (set `self.AmmoGainTagCont` (struct :`GameplayTags` (struct :`(TagName` "Pickup.Ammo.Shotgun.Shells.Large"))))))
    (`AbilitySystemComponent.TryActivateAbilitiesByTag` (`self.AbilitySystemComponent`) (`self.AmmoGainTagCont`) true)
    (`self.ItemPickup`)))

(fn `GetWeaponFromDT`
  (params (Weapon :type "/Game/OldSchoolFPS/Blueprints/Enums/ENUM_WeaponList Enum" :default "NewEnumerator0"))
  (returns (WeaponData :type "/Game/OldSchoolFPS/Blueprints/Structs/ST_WeaponData Structure") (WeaponFound :type Boolean))
  (locals (WeaponExists :type Boolean) (WeaponToEquip :type "/Game/OldSchoolFPS/Blueprints/Structs/ST_WeaponData Structure"))
  (bind _outrownames (`DataTableFunctionLibrary.GetDataTableRowNames` "/Game/OldSchoolFPS/Blueprints/Weapons/DT_OSFPSWeapons.DT_OSFPSWeapons"))
  (for _array_element _outrownames
    (bind _returnvalue (`|GetDataTableRow` "/Game/OldSchoolFPS/Blueprints/Weapons/DT_OSFPSWeapons.DT_OSFPSWeapons" _array_element)
      (:`then`
        (if (`|EnumEquality` Weapon (`.WeaponName_3_853D30BD40417274EB9F7F9266644A8D` (break `/Game/OldSchoolFPS/Blueprints/Structs/ST_WeaponData` _returnvalue)))
          (set `local.WeaponExists` true)
          (set `local.WeaponToEquip` _returnvalue)
          (break)))))
  (return (`local.WeaponToEquip`) (`local.WeaponExists`)))

(fn `HasWeapon`
  (params (ST_WeaponData :type "/Game/OldSchoolFPS/Blueprints/Enums/ENUM_WeaponList Enum" :default "NewEnumerator0"))
  (returns (`HasWeapon?` :type Boolean))
  (locals (HasWeapon :type Boolean))
  (for _array_element (`self.PlayerWeapons`)
    (if (`|EnumEquality` (`.WeaponName_3_853D30BD40417274EB9F7F9266644A8D` (break `/Game/OldSchoolFPS/Blueprints/Structs/ST_WeaponData` _array_element)) ST_WeaponData)
      (set `local.HasWeapon` true)
      (break)))
  (return (`local.HasWeapon`)))

(fn `InitWeapon`
  (params (`In Class` :type "/Game/OldSchoolFPS/Blueprints/Player/BP_PlayerWeaponBase Class Reference"))
  (returns (WeaponActor :type "Actor Object Reference"))
  (bind _weapon (`self.Weapon`))
  (bind _childactor (`ChildActorComponent.ChildActor` _weapon))
  (`ChildActorComponent.SetChildActorClass` _weapon `In Class`)
  (if (`KismetSystemLibrary.DoesImplementInterface` _childactor "/Game/OldSchoolFPS/Blueprints/Interfaces/I_PlayerWeapon.I_PlayerWeapon_C")
    (message `/Game/OldSchoolFPS/Blueprints/Interfaces/I_PlayerWeapon.InitWeapon` _childactor))
  (return _childactor))

(fn `UpdateUI`
  (bind _abilitysystemcomponent (`self.AbilitySystemComponent`))
  (bind _hud (`self.HUD`))
  (bind _hud_2 (`self.HUD`))
  (bind _abilitysystemcomponent_2 (`self.AbilitySystemComponent`))
  (`TextBlock.SetText` (`/Game/OldSchoolFPS/Blueprints/Widgets/HUD.HealthValue` _hud) (`KismetTextLibrary.Conv_DoubleToText` (`.ReturnValue` (`AbilitySystemBlueprintLibrary.GetFloatAttributeFromAbilitySystemComponent` _abilitysystemcomponent (struct :`AttributeName` "Health" :`Attribute` "/Script/OldSchoolFPS.OSFPSAttributeSet:Health" :`AttributeOwner` "/Script/CoreUObject.Class'\"/Script/OldSchoolFPS.OSFPSAttributeSet\"'"))) "HalfToEven"))
  (`TextBlock.SetText` (`/Game/OldSchoolFPS/Blueprints/Widgets/HUD.ArmorValue` _hud) (`KismetTextLibrary.Conv_DoubleToText` (`.ReturnValue` (`AbilitySystemBlueprintLibrary.GetFloatAttributeFromAbilitySystemComponent` _abilitysystemcomponent (struct :`AttributeName` "Armour" :`Attribute` "/Script/OldSchoolFPS.OSFPSAttributeSet:Armour" :`AttributeOwner` "/Script/CoreUObject.Class'\"/Script/OldSchoolFPS.OSFPSAttributeSet\"'"))) "HalfToEven"))
  (switch `/Game/OldSchoolFPS/Blueprints/Enums/ENUM_AmmoList` (`.AmmoType_11_32F3369F42A6AE46665E4EA199FF75E0` (break `/Game/OldSchoolFPS/Blueprints/Structs/ST_WeaponData` (`self.CurrentWeapon`)))
    (:`NewEnumerator1`
      (`TextBlock.SetText` (`/Game/OldSchoolFPS/Blueprints/Widgets/HUD.PistolAmmoValue` _hud_2) (`KismetTextLibrary.Conv_DoubleToText` (`.ReturnValue` (`AbilitySystemBlueprintLibrary.GetFloatAttributeFromAbilitySystemComponent` _abilitysystemcomponent_2 (struct :`AttributeName` "Bullets" :`Attribute` "/Script/OldSchoolFPS.OSFPSAttributeSet:Bullets" :`AttributeOwner` "/Script/CoreUObject.Class'\"/Script/OldSchoolFPS.OSFPSAttributeSet\"'"))) "HalfToEven")))
    (:`NewEnumerator2`
      (`TextBlock.SetText` (`/Game/OldSchoolFPS/Blueprints/Widgets/HUD.RocketAmmoValue` _hud_2) (`KismetTextLibrary.Conv_DoubleToText` (`.ReturnValue` (`AbilitySystemBlueprintLibrary.GetFloatAttributeFromAbilitySystemComponent` _abilitysystemcomponent_2 (struct :`AttributeName` "Rockets" :`Attribute` "/Script/OldSchoolFPS.OSFPSAttributeSet:Rockets" :`AttributeOwner` "/Script/CoreUObject.Class'\"/Script/OldSchoolFPS.OSFPSAttributeSet\"'"))) "HalfToEven")))
    (:`NewEnumerator3`
      (`TextBlock.SetText` (`/Game/OldSchoolFPS/Blueprints/Widgets/HUD.ShotgunAmmoValue` _hud_2) (`KismetTextLibrary.Conv_DoubleToText` (`.ReturnValue` (`AbilitySystemBlueprintLibrary.GetFloatAttributeFromAbilitySystemComponent` _abilitysystemcomponent_2 (struct :`AttributeName` "Shells" :`Attribute` "/Script/OldSchoolFPS.OSFPSAttributeSet:Shells" :`AttributeOwner` "/Script/CoreUObject.Class'\"/Script/OldSchoolFPS.OSFPSAttributeSet\"'"))) "HalfToEven")))))

(fn `UserConstructionScript`)