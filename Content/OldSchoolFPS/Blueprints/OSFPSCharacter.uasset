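; Character Blueprint for an old-school FPS that handles taking damage and death through the Gameplay Ability System.
; TakeDamage receives gameplay cue data and reports a damage event with the instigator and hit location, as used by AI damage sensing.
; It then runs HealthCheck, which tests an ability system attribute against zero, and calls KillCharacter on depletion.
; KillCharacter is an empty event here, and the health and armour debug prints are disconnected.
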(event `self.ReceiveBeginPlay`)

(event `TakeDamage`
  (params (CueData :type "GameplayCueParameters Structure"))
  (bind (_normalizedmagnitude _rawmagnitude _effectcontext _matchedtagname _originaltag _aggregatedsourcetags _aggregatedtargettags _location) (`AbilitySystemBlueprintLibrary.BreakGameplayCueParameters` CueData))
  (`AISense_Damage.ReportDamageEvent` self (`AbilitySystemBlueprintLibrary.EffectContextGetInstigatorActor` _effectcontext) 0.0 _location)
  (if (`self.HealthCheck`)
    (`self.KillCharacter`)))

(event `KillCharacter`)

(fn `HealthCheck`
  (returns (IsDead :type Boolean))
  (return (<= (`.ReturnValue` (`AbilitySystemBlueprintLibrary.GetFloatAttributeFromAbilitySystemComponent` (`self.AbilitySystemComponent`) (struct :`AttributeName` "Health" :`Attribute` "/Script/OldSchoolFPS.OSFPSAttributeSet:Health" :`AttributeOwner` "/Script/CoreUObject.Class'\"/Script/OldSchoolFPS.OSFPSAttributeSet\"'"))) 0.0)))

(fn `UserConstructionScript`)