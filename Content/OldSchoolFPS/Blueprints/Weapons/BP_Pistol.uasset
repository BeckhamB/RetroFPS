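; BP_Pistol is the player's pistol in an old-school FPS, drawn as an animated Paper2D flipbook.
; InitWeapon shows the idle flipbook and caches the player pawn as BP_FPCC.
; ShootPistol flashes a point light, plays the gun sound, updates the player's UI and runs the fire flipbook for its length before returning to idle.
; It handles only presentation, with no hit or damage logic in these graphs.
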(event `/Game/OldSchoolFPS/Blueprints/Interfaces/I_PlayerWeapon.InitWeapon`
  (`PaperFlipbookComponent.SetFlipbook` (`self.WeaponFlipbook`) (`self.IdlePistol`))
  (`SceneComponent.SetHiddenInGame` (`self.WeaponFlipbook`) false false)
  (bind _asbp_fpcc (cast `/Game/OldSchoolFPS/Blueprints/Player/BP_FPCC` (`GameplayStatics.GetPlayerPawn` 0)))
  (set `self.As BP FPCC` _asbp_fpcc))

(event `ShootPistol`
  (bind _weaponflipbook (`self.WeaponFlipbook`))
  (`self.LightFlash`)
  (`GameplayStatics.PlaySound2D` "/Game/OldSchoolFPS/Audio/Weapons/pistol.pistol" 1.0 1.0 0.0 null null)
  (`/Game/OldSchoolFPS/Blueprints/Player/BP_FPCC.UpdateUI` (`self.As BP FPCC`))
  (`PaperFlipbookComponent.SetFlipbook` _weaponflipbook (`self.FirePistol`))
  (`KismetSystemLibrary.Delay` (`PaperFlipbookComponent.GetFlipbookLength` _weaponflipbook))
  (`PaperFlipbookComponent.SetFlipbook` (`self.WeaponFlipbook`) (`self.IdlePistol`)))

(event `LightFlash`
  (bind _pointlight (`self.PointLight`))
  (`SceneComponent.SetHiddenInGame` _pointlight false false)
  (`KismetSystemLibrary.Delay` 0.25)
  (`SceneComponent.SetHiddenInGame` _pointlight true false))

(fn `UserConstructionScript`
  (`parent.UserConstructionScript`))