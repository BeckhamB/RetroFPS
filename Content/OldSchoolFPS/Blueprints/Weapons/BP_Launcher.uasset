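; Rocket launcher weapon for an old-school FPS, drawn as an animated flipbook with idle and fire animations.
; InitWeapon shows the idle flipbook and caches the BP_FPCC player pawn.
; ShootLauncher plays the fire sound, briefly flashes a point light, refreshes the player's UI and spawns a BP_Rocket at the Sphere component's transform.
; The fire flipbook then plays for its own length before returning to idle.
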(event `/Game/OldSchoolFPS/Blueprints/Interfaces/I_PlayerWeapon.InitWeapon`
  (`PaperFlipbookComponent.SetFlipbook` (`self.WeaponFlipbook`) (`self.IdleLauncher`))
  (`SceneComponent.SetHiddenInGame` (`self.WeaponFlipbook`) false false)
  (bind _asbp_fpcc (cast `/Game/OldSchoolFPS/Blueprints/Player/BP_FPCC` (`GameplayStatics.GetPlayerPawn` 0)))
  (set `self.As BP FPCC` _asbp_fpcc))

(event `ShootLauncher`
  (bind _weaponflipbook (`self.WeaponFlipbook`))
  (`GameplayStatics.PlaySound2D` "/Game/OldSchoolFPS/Audio/Weapons/launcherFire.launcherFire" 1.0 1.0 0.0 null null)
  (`self.LightFlash`)
  (`/Game/OldSchoolFPS/Blueprints/Player/BP_FPCC.UpdateUI` (`self.As BP FPCC`))
  (`|SpawnActorFromClass` "/Game/OldSchoolFPS/Blueprints/Abilities/Launcher/BP_Rocket.BP_Rocket_C" (`SceneComponent.K2_GetComponentToWorld` (`self.Sphere`)) "Undefined" "OverrideRootScale" null null)
  (`PaperFlipbookComponent.SetFlipbook` _weaponflipbook (`self.FireLauncher`))
  (`KismetSystemLibrary.Delay` (`PaperFlipbookComponent.GetFlipbookLength` _weaponflipbook))
  (`PaperFlipbookComponent.SetFlipbook` (`self.WeaponFlipbook`) (`self.IdleLauncher`)))

(event `LightFlash`
  (bind _pointlight (`self.PointLight`))
  (`SceneComponent.SetHiddenInGame` _pointlight false false)
  (`KismetSystemLibrary.Delay` 0.25)
  (`SceneComponent.SetHiddenInGame` _pointlight true false))

(fn `UserConstructionScript`
  (`parent.UserConstructionScript`))