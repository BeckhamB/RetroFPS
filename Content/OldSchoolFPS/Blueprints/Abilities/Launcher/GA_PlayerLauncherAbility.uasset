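; Gameplay ability that fires the player's rocket launcher in the old-school FPS.
; FireWeapon checks that an ability system attribute is above zero, applies the rocket-spend effect, then calls ShootLauncher on the weapon.
; Helpers lazily cache the player and the launcher from the weapon child actor.
; An uncalled GetLineTrace helper traces from the camera, returning the hit actor or otherwise placing a pooled object at the impact point.
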(event `self.FireWeapon`
  (bind _playerlauncherweaponcomp (`self.PlayerLauncherWeaponComp`))
  (`self.GetPlayer`)
  (if (> (`.ReturnValue` (`AbilitySystemBlueprintLibrary.GetFloatAttributeFromAbilitySystemComponent` (`AbilitySystemBlueprintLibrary.GetAbilitySystemComponent` (`self.Player`)) (struct :`AttributeName` "Rockets" :`Attribute` "/Script/OldSchoolFPS.OSFPSAttributeSet:Rockets" :`AttributeOwner` "/Script/CoreUObject.Class'\"/Script/OldSchoolFPS.OSFPSAttributeSet\"'"))) 0.0)
    (`self.GetWeapon`)
    (`/Engine/EditorBlueprintResources/StandardMacros.IsValid` _playerlauncherweaponcomp
      (:`Is Valid`
        (`self.BP_ApplyGameplayEffectToOwner` "/Game/OldSchoolFPS/Blueprints/Abilities/Launcher/GE_PlayerRocketSpend.GE_PlayerRocketSpend_C")
        (`/Game/OldSchoolFPS/Blueprints/Weapons/BP_Launcher.ShootLauncher` _playerlauncherweaponcomp)))))

(fn `GetLineTrace`
  (returns (Actor :type "Actor Object Reference"))
  (bind _camera (`/Game/OldSchoolFPS/Blueprints/Player/BP_FPCC.Camera` (`self.Player`)))
  (bind _returnvalue (`SceneComponent.K2_GetComponentLocation` _camera))
  (bind _outhit (`KismetSystemLibrary.LineTraceSingle` _returnvalue (+ _returnvalue (* (`KismetMathLibrary.GetForwardVector` (`SceneComponent.K2_GetComponentRotation` _camera)) (`self.WeaponRange`))) "TraceTypeQuery1"))
  (bind (_bblockinghit _binitialoverlap _time _distance _location _impactpoint _normal _impactnormal _physmat _hitactor) (`GameplayStatics.BreakHitResult` _outhit))
  (`/Engine/EditorBlueprintResources/StandardMacros.IsValid` _hitactor
    (:`Is Valid`
      (return _hitactor))
    (:`Is Not Valid`
      (bind _returnvalue_2 (`ObjectPooling.SpawnPooledObject` (`/Game/OldSchoolFPS/Blueprints/Player/BP_FPCC.ObjectPooling` (`self.Player`))))
      (`Actor.K2_SetActorLocation` _returnvalue_2 _impactpoint false false)
      (`Actor.K2_SetActorRotation` _returnvalue_2 (`KismetMathLibrary.Conv_VectorToRotator` _impactnormal) false))))

(fn `GetPlayer`
  (bind _returnvalue_owneractor (break `GameplayAbilityActorInfo` (`self.GetActorInfo`)))
  (`/Engine/EditorBlueprintResources/StandardMacros.IsValid` (`self.Player`)
    (:`Is Valid`
      _)
    (:`Is Not Valid`
      (bind _asbp_fpcc (cast `/Game/OldSchoolFPS/Blueprints/Player/BP_FPCC` _returnvalue_owneractor))
      (set `self.Player` _asbp_fpcc)))
  (return))

(fn `GetWeapon`
  (`/Engine/EditorBlueprintResources/StandardMacros.IsValid` (`self.PlayerLauncherWeaponComp`)
    (:`Is Valid`
      _)
    (:`Is Not Valid`
      (bind _asbp_launcher (cast `/Game/OldSchoolFPS/Blueprints/Weapons/BP_Launcher` (`ChildActorComponent.ChildActor` (`/Game/OldSchoolFPS/Blueprints/Player/BP_FPCC.Weapon` (`self.Player`)))))
      (set `self.PlayerLauncherWeaponComp` _asbp_launcher)))
  (return))