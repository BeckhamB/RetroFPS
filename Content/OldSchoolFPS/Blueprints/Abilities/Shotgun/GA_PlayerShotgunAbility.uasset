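; Player shotgun gameplay ability that fires one camera-forward hitscan shot when a checked ability-system attribute is above zero.
; FireWeapon caches the player and shotgun, applies the spend effect, calls ShootShotgun, then line traces on Visibility.
; A hit OSFPSCharacter receives ApplyEffect and the shotgun damage GameplayEffect through its own ability system.
; When the trace returns no valid actor, a pooled object is placed at the impact point, aligned to the normal.
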(event `self.FireWeapon`
  (bind _shotgunweaponcomp (`self.ShotgunWeaponComp`))
  (`self.GetPlayer`)
  (if (> (`.ReturnValue` (`AbilitySystemBlueprintLibrary.GetFloatAttributeFromAbilitySystemComponent` (`AbilitySystemBlueprintLibrary.GetAbilitySystemComponent` (`self.Player`)) (struct :`AttributeName` "Shells" :`Attribute` "/Script/OldSchoolFPS.OSFPSAttributeSet:Shells" :`AttributeOwner` "/Script/CoreUObject.Class'\"/Script/OldSchoolFPS.OSFPSAttributeSet\"'"))) 0.0)
    (`self.GetWeapon`)
    (`/Engine/EditorBlueprintResources/StandardMacros.IsValid` _shotgunweaponcomp
      (:`Is Valid`
        (`self.BP_ApplyGameplayEffectToOwner` "/Game/OldSchoolFPS/Blueprints/Abilities/Shotgun/GE_PlayerShotgunSpend.GE_PlayerShotgunSpend_C")
        (`/Game/OldSchoolFPS/Blueprints/Weapons/BP_Shotgun.ShootShotgun` _shotgunweaponcomp)
        (bind _actor (`self.GetLineTrace`))
        (bind _asosfpscharacter (cast `OSFPSCharacter` _actor))
        (`self.ApplyEffect` (`self.Player`) _asosfpscharacter)
        (bind _returnvalue (`AbilitySystemBlueprintLibrary.GetAbilitySystemComponent` _asosfpscharacter))
        (`AbilitySystemComponent.BP_ApplyGameplayEffectToTarget` _returnvalue "/Game/OldSchoolFPS/Blueprints/Abilities/Shotgun/GE_PlayerShotgunDamage.GE_PlayerShotgunDamage_C" _returnvalue 0.0 (`AbilitySystemComponent.MakeEffectContext` _returnvalue))))))

(fn `GetLineTrace`
  (returns (Actor :type "Actor Object Reference"))
  (bind _camera (`/Game/OldSchoolFPS/Blueprints/Player/BP_FPCC.Camera` (`self.Player`)))
  (bind _returnvalue (`SceneComponent.K2_GetComponentLocation` _camera))
  (bind _outhit (`KismetSystemLibrary.LineTraceSingle` _returnvalue (+ _returnvalue (* (`KismetMathLibrary.GetForwardVector` (`SceneComponent.K2_GetComponentRotation` _camera)) (`self.WeaponRange`))) "TraceTypeQuery1"))
  (bind (_bblockinghit _binitialoverlap _time _distance _location _impactpoint _normal _impactnormal _physmat _hitactor) (`GameplayStatics.BreakHitResult` _outhit))
  (`/Engine/EditorBlueprintResources/StandardMacros.IsValid` _hitactor
    (:`Is Valid`
      (return _hitactor))
    (:`Is Not Valid`
      (bind _returnvalue_2 (`ObjectPooling.SpawnPooledObject` (`/Game/OldSchoolFPS/Blueprints/Player/BP_FPCC.ObjectPooling` (`self.Player`))))
      (`Actor.K2_SetActorLocation` _returnvalue_2 _impactpoint false false)
      (`Actor.K2_SetActorRotation` _returnvalue_2 (`KismetMathLibrary.Conv_VectorToRotator` _impactnormal) false))))

(fn `GetPlayer`
  (bind _returnvalue_owneractor (break `GameplayAbilityActorInfo` (`self.GetActorInfo`)))
  (`/Engine/EditorBlueprintResources/StandardMacros.IsValid` (`self.Player`)
    (:`Is Valid`
      _)
    (:`Is Not Valid`
      (bind _asbp_fpcc (cast `/Game/OldSchoolFPS/Blueprints/Player/BP_FPCC` _returnvalue_owneractor))
      (set `self.Player` _asbp_fpcc)))
  (return))

(fn `GetWeapon`
  (`/Engine/EditorBlueprintResources/StandardMacros.IsValid` (`self.ShotgunWeaponComp`)
    (:`Is Valid`
      _)
    (:`Is Not Valid`
      (bind _asbp_shotgun (cast `/Game/OldSchoolFPS/Blueprints/Weapons/BP_Shotgun` (`ChildActorComponent.ChildActor` (`/Game/OldSchoolFPS/Blueprints/Player/BP_FPCC.Weapon` (`self.Player`)))))
      (set `self.ShotgunWeaponComp` _asbp_shotgun)))
  (return))