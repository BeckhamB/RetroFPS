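; Boss enemy weapon ability that fires a hitscan shot at player characters.
; FireWeapon caches the owning BossEnemy, then runs a Visibility line trace forward from its capsule out to WeaponRange.
; If the hit actor is an OSFPSCharacter, it calls ApplyEffect with the boss as attacker and that character as target.
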(event `self.FireWeapon`
  (`self.GetEnemy`)
  (bind _actor (`self.Get Line Trace`))
  (bind _asosfpscharacter (cast `/Game/OldSchoolFPS/Blueprints/OSFPSCharacter` _actor))
  (`self.ApplyEffect` (`self.BossEnemy`) _asosfpscharacter))

(fn `Get Line Trace`
  (returns (Actor :type "Actor Object Reference"))
  (bind _capsulecomponent (`Character.CapsuleComponent` (`self.BossEnemy`)))
  (bind _returnvalue (`SceneComponent.K2_GetComponentLocation` _capsulecomponent))
  (bind _outhit (`KismetSystemLibrary.LineTraceSingle` _returnvalue (+ _returnvalue (* (`KismetMathLibrary.GetForwardVector` (`SceneComponent.K2_GetComponentRotation` _capsulecomponent)) (`self.WeaponRange`))) "TraceTypeQuery1"))
  (bind (_bblockinghit _binitialoverlap _time _distance _location _impactpoint _normal _impactnormal _physmat _hitactor) (`GameplayStatics.BreakHitResult` _outhit))
  (`/Engine/EditorBlueprintResources/StandardMacros.IsValid` _hitactor
    (:`Is Valid`
      (return _hitactor))))

(fn `GetEnemy`
  (bind _returnvalue_owneractor (break `GameplayAbilityActorInfo` (`self.GetActorInfo`)))
  (`/Engine/EditorBlueprintResources/StandardMacros.IsValid` (`self.BossEnemy`)
    (:`Is Valid`
      _)
    (:`Is Not Valid`
      (bind _asboss_enemy (cast `/Game/OldSchoolFPS/Blueprints/Enemies/BossEnemy` _returnvalue_owneractor))
      (set `self.BossEnemy` _asboss_enemy)))
  (return))