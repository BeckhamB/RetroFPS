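; Gameplay ability that fires the pistol enemy's hitscan shot at the player character class.
; FireWeapon caches the owning BP_PistolEnemy, then line-traces on Visibility from its capsule along the forward vector for WeaponRange.
; A hit BP_OSFPSCharacter receives an effect through ApplyEffect.
; When the trace returns no valid actor, an object from the enemy's pool is placed at the impact point, aligned to the normal.
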(event `self.FireWeapon`
  (`self.GetEnemy`)
  (bind _actor (`self.GetLineTrace`))
  (bind _asbp_osfpscharacter (cast `/Game/OldSchoolFPS/Blueprints/BP_OSFPSCharacter` _actor))
  (`self.ApplyEffect` (`self.PistolEnemy`) _asbp_osfpscharacter))

(fn `GetEnemy`
  (bind _returnvalue_owneractor (break `GameplayAbilityActorInfo` (`self.GetActorInfo`)))
  (`/Engine/EditorBlueprintResources/StandardMacros.IsValid` (`self.PistolEnemy`)
    (:`Is Valid`
      _)
    (:`Is Not Valid`
      (bind _asbp_pistol_enemy (cast `/Game/OldSchoolFPS/Blueprints/Enemies/BP_PistolEnemy` _returnvalue_owneractor))
      (set `self.PistolEnemy` _asbp_pistol_enemy)))
  (return))

(fn `GetLineTrace`
  (returns (Actor :type "Actor Object Reference"))
  (bind _capsulecomponent (`Character.CapsuleComponent` (`self.PistolEnemy`)))
  (bind _returnvalue (`SceneComponent.K2_GetComponentLocation` _capsulecomponent))
  (bind _outhit (`KismetSystemLibrary.LineTraceSingle` _returnvalue (+ _returnvalue (* (`KismetMathLibrary.GetForwardVector` (`SceneComponent.K2_GetComponentRotation` _capsulecomponent)) (`self.WeaponRange`))) "TraceTypeQuery1"))
  (bind (_bblockinghit _binitialoverlap _time _distance _location _impactpoint _normal _impactnormal _physmat _hitactor) (`GameplayStatics.BreakHitResult` _outhit))
  (`/Engine/EditorBlueprintResources/StandardMacros.IsValid` _hitactor
    (:`Is Valid`
      (return _hitactor))
    (:`Is Not Valid`
      (bind _returnvalue_2 (`ObjectPooling.SpawnPooledObject` (`/Game/OldSchoolFPS/Blueprints/Enemies/BP_PistolEnemy.ObjectPooling` (`self.PistolEnemy`))))
      (`Actor.K2_SetActorLocation` _returnvalue_2 _impactpoint false false)
      (`Actor.K2_SetActorRotation` _returnvalue_2 (`KismetMathLibrary.Conv_VectorToRotator` _impactnormal) false))))